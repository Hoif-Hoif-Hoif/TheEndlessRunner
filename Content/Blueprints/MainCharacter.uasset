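; MainCharacter is the player character Blueprint, handling jumping, a time-based score, lives and game over.
; BeginPlay switches to game-only input, shows the score widget and starts a looping timer that raises the score while alive.
; A DoOnce gate allows one jump until landing resets it.
; PlayerDie removes health and updates the widget, or at zero shows the game-over widget and pauses after a short delay.
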(event `self.ReceiveBeginPlay`
  (bind _returnvalue (`GameplayStatics.GetPlayerController` 0))
  (set `PlayerController.bShowMouseCursor` false _returnvalue)
  (`WidgetBlueprintLibrary.SetInputMode_GameOnly` _returnvalue)
  (bind _returnvalue_2 (`|CreateWidget` "/Game/Blueprints/ScoreWidget.ScoreWidget_C"))
  (bind _output_get (set `self.score` _returnvalue_2))
  (`UserWidget.AddToViewport` _output_get 0)
  (`KismetSystemLibrary.K2_SetTimerDelegate` (delegate `UpdateScore`) 1.0 true))

(event `UpdateScore`
  (if (not (`self.isDead`))
    (bind _result (`/Engine/EditorBlueprintResources/StandardMacros.IncrementInt` (`self.scoreInt`))
      (:`  `
        (`/Game/Blueprints/ScoreWidget.UpdateScore` (`self.score`) _result)))))

(event `InputAction|action_jump`
  (params (Key :type "Key Structure"))
  (:`Pressed`
    (if (not (`self.isDead`))
      (`/Engine/EditorBlueprintResources/StandardMacros.DoOnce` false :!label _label
        (:`Completed`
          (`self.Jump`))))))

(event `self.OnLanded`
  (params (Hit :type "HitResult Structure (by ref)"))
  (goto _label :!via `Reset`))

(event `PlayerDie`
  (bind _result (`/Engine/EditorBlueprintResources/StandardMacros.DecrementInt` (`self.healthInt`))
    (:`  `
      (if (== _result 0)
        (set `self.isDead` true)
        (bind _returnvalue (`|CreateWidget` "/Game/Blueprints/GameOverWidget.GameOverWidget_C"))
        (`UserWidget.AddToViewport` _returnvalue 0)
        (`KismetSystemLibrary.Delay` 0.2)
        (`GameplayStatics.SetGamePaused` true)
        (else
          (`/Game/Blueprints/ScoreWidget.UpdateHealth` (`self.score`) (`self.healthInt`)))))))

(fn `UserConstructionScript`)