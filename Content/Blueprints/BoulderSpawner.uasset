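; Spawner actor that creates Boulders at its Scene component's transform and spawns them more reliably over time.
; BeginPlay starts a looping timer with a random interval picked once.
; Each tick of that timer rolls a random value between DifficultyModifier and 2, truncates it, and spawns only on 1 or 2.
; Each spawn nudges DifficultyModifier upward, narrowing the roll toward guaranteed spawns.
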(event `self.ReceiveBeginPlay`
  (`KismetSystemLibrary.K2_SetTimerDelegate` (delegate `SpawnBoulder`) (`KismetMathLibrary.RandomFloatInRange` 0.25 2.5) true))

(event `SpawnBoulder`
  (switch `int` (`KismetMathLibrary.Conv_Int64ToInt` (`KismetMathLibrary.Conv_DoubleToInt64` (`KismetMathLibrary.RandomFloatInRange` (`self.difficultyModifier`) 2.0)))
    (:`1`
      _)
    (:`2`
      _))
  (`|SpawnActorFromClass` "/Game/Blueprints/Boulder.Boulder_C" (`SceneComponent.K2_GetComponentToWorld` (`self.Scene`)) "Undefined" "OverrideRootScale" null null)
  (`self.IncreaseDifficulty`))

(event `IncreaseDifficulty`
  (set `self.difficultyModifier` (- (`self.difficultyModifier`) -0.01)))

(fn `UserConstructionScript`)